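; DodgeLaser is a laser hazard actor for a dodge-laser game mode that either scores points or damages the player.
; On collision overlap, a ScoreTag actor makes it add its score amount through DodgeLaserMode.
; A Player-tagged actor instead triggers a hurt sound and damage calculation on the ThirdPersonCharacter.
; The laser destroys itself after either outcome; no movement logic appears in this graph.
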(event `self.LaserCollision.OnComponentBeginOverlap`
  (params (OverlappedComponent :type "PrimitiveComponent Object Reference") (OtherActor :type "Actor Object Reference") (OtherComp :type "PrimitiveComponent Object Reference") (OtherBodyIndex :type Integer) (bFromSweep :type Boolean) (SweepResult :type "HitResult Structure (by ref)"))
  ;[1 1 1] Check if collides with player or scoretrigger
  (if (`self.ActorHasTag` OtherActor "ScoreTag")
    (bind _asdodge_laser_mode (cast `/Game/BluePrints/DodgeLaserMode` (`GameplayStatics.GetGameMode`)))
    (`/Game/BluePrints/DodgeLaserMode.IncreaseScore` _asdodge_laser_mode (`self.ScoreAmount`))
    (`self.K2_DestroyActor`)
    (elif (`self.ActorHasTag` OtherActor "Player")
      (`GameplayStatics.SpawnSoundAttached` "/Game/AudioFiles/Hit_Hurt10.Hit_Hurt10" (`self.LaserCollision`) "None" (0.0 0.0 0.0) (struct) "KeepRelativeOffset" false 1.0 1.0 0.0 null null)
      (bind _asthird_person_character (cast `/Game/BluePrints/ThirdPersonCharacter` OtherActor))
      (`/Game/BluePrints/ThirdPersonCharacter.CalculateDamage` _asthird_person_character)
      (`self.K2_DestroyActor`))))

(fn `UserConstructionScript`)