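; Spawner actor that fires DodgeLaser actors from random LaserSpawnPoint locations while the player is alive.
; BeginPlay caches all spawn points, then starts a delay-driven loop between LaserSpawnControl and SpawnDodgeLasers that stops once the ThirdPersonCharacter is dead.
; A parallel recursive timer periodically shortens the firing delay down to a floor, steadily raising difficulty, and ResetTimer restores the starting interval.
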(event `SpawnDodgeLasers`
  ;[1 1 1] Randomize the dodge laser spawning point
  (`|SpawnActorFromClass` "/Game/BluePrints/DodgeLaser.DodgeLaser_C" (`self.GetTransform` (`|GetArrayItem` (`self.LaserSpawnArray`) (`KismetMathLibrary.RandomInteger` (`self.LaserArrayLength`)))) "Undefined" "OverrideRootScale" null null)
  (`self.LaserSpawnControl`))

(event `LaserSpawnControl`
  ;[1 1 1] Shoot lasers if player is alive
  (`KismetSystemLibrary.Delay` (`self.LaserShootTimer`))
  (bind _asthird_person_character (cast `/Game/BluePrints/ThirdPersonCharacter` (`GameplayStatics.GetPlayerCharacter` 0)))
  (if (not (`/Game/BluePrints/ThirdPersonCharacter.IsPlayerDead` _asthird_person_character))
    (`self.SpawnDodgeLasers`)))

(event `TimerDecrease`
  ;[1 1 1] Decrease the laser shooting timer until some point
  (`KismetSystemLibrary.Delay` 5.0)
  (if (> (`self.LaserShootTimer`) 0.2)
    (set `self.LaserShootTimer` (* (`self.LaserShootTimer`) 0.95))
    (`self.TimerDecrease`)))

(event `self.ReceiveBeginPlay`
  ;[1 1 1] Setup for other functions
  (`|ExecutionSequence`
    (:`then_0`
      (bind _outactors (`GameplayStatics.GetAllActorsOfClass` "/Game/BluePrints/LaserSpawnPoint.LaserSpawnPoint_C"))
      (bind _output_get (set `self.LaserSpawnArray` _outactors))
      (set `self.LaserArrayLength` (`KismetArrayLibrary.Array_Length` _output_get)))
    (:`then_1`
      (`self.LaserSpawnControl`))
    (:`then_2`
      (`self.TimerDecrease`))))

(event `ResetTimer`
  ;[1 1 1] Reset the laser shooting timer
  (set `self.LaserShootTimer` 2.0))

(fn `UserConstructionScript`)